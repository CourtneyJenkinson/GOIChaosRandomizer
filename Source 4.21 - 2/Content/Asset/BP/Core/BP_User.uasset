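; Player pawn for a top-down randomizer that shuffles crew and spectators into grouped column slots, using an orthographic camera with key and widget pan/zoom.
; The construction script caches crew, spectator and Petri actors, and each randomize trigger reshuffles and repositions them using DoOnce/DoN counters for spacing.
; The x10/x100/x1000 inputs only scale the press counter.
; It also caps FPS, toggles PastaMode audio and logo, and shows or hides Petri pilots by Z offset.
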(event `self.ReceiveBeginPlay`
  ;[1 1 1] Event BeginPlay
  (`|ExecutionSequence`
    (:`then_0`
      (`KismetSystemLibrary.ExecuteConsoleCommand` "t.maxfps 15") ; Sets fps to 10 frames per second
      (`AudioComponent.Stop` (`self.Audio`)))
    (:`then_1`
      (set `self.OrthoWidth` (`CameraComponent.OrthoWidth` (`self.Camera`))) ; Grabs ortho width to be used as base ref for UI zooming
    )))

(event `InputAction|PastaMode`
  (params (Key :type "Key Structure"))
  (bind _pastalogo (`self.PastaLogo`))
  ;[1 0.7712 0] Set Modes
  ;;[1 1 1] PastaMode Toggle
  (:`Pressed`
    (if (`self.PastaMode`)
      (`AudioComponent.Play` (`self.Audio`) 0.0)
      (`PrimitiveComponent.SetMaterial` _pastalogo 0 "/Game/Asset/Art/Mat/PastaLogo_Mat_Inst1.PastaLogo_Mat_Inst1")
      (set `self.PastaMode` false)
      (else
        (`AudioComponent.Stop` (`self.Audio`))
        (`PrimitiveComponent.SetMaterial` _pastalogo 0 "/Game/Asset/Art/Mat/PastaLogo_Mat_Inst.PastaLogo_Mat_Inst")
        (set `self.PastaMode` true)))))

(event `InputAction|RandomizeReset`
  (params (Key :type "Key Structure"))
  ;[1 0.7712 0] Set Modes
  ;;[1 1 1] Reset Button Count Trigger
  (:`Pressed`
    (set `self.ButtonCount` 0)))

(event `InputAxis|MoveForward` :overrideparent false
  (params (AxisValue :type "Float (single-precision)"))
  ;[1 1 1] Movement
  ;;[0 1 0.003035] Panning With Keyboard
  (`self.AddMovementInput` (`KismetMathLibrary.GetForwardVector` (`KismetMathLibrary.MakeRotator` 0.0 0.0 (.yaw (`self.GetControlRotation`)))) AxisValue))

(event `Spectator Randomizer`
  (bind _output (`|GetArrayItem` (`self.SpecArray`) (`self.CurrentIndex_Spectate`)))
  ;[0.2785 0 1] Randomize Spectators
  ;;[1 1 1] Reset variables
  (set `self.CurrentIndex_Spectate` 0)
  (set `self.SpecPosition` (0.0 730.0 0.0))
  (`KismetArrayLibrary.Array_Shuffle` (`self.SpecArray`))
  (for _index (range (+ (`KismetArrayLibrary.Array_LastIndex` (`self.SpecArray`)) 1))
    (set `self.CurrentIndex_Spectate` _index)
    (`|ExecutionSequence`
      (:`then_0`
        ;;[1 1 1] Set Spector into slot position
        (`self.K2_SetActorLocation` _output (+ (`self.SpecPosition`) (`self.VectorIteration_Spectate`)) false false)
        (set `self.SpecPosition` (`self.K2_GetActorLocation` _output)))
      (:`then_1`
        ;;[1 1 1] Sorts Spectators into columns
        (if (>= (`self.CurrentIndex_Spectate`) 1)
          (`/Engine/EditorBlueprintResources/StandardMacros.DoOnce` false :!label _label
            (:`Completed`
              (set `self.SpecPosition` (300.0 725.0 0.0))))
          (else
            (`/Engine/EditorBlueprintResources/StandardMacros.DoOnce` false))))
      (:`then_2`
        ;;[1 1 1] Sort Spectator into slots
        (if (!= (`self.SpecIter`) 1)
          (bind _counter (`/Engine/EditorBlueprintResources/StandardMacros.Do N` 1)
            (:`Exit`
              (set `self.SpecIter` _counter)
              (set `self.VectorIteration_Spectate` (`KismetMathLibrary.MakeVector` (.x (`self.VectorIteration_Spectate`)) 25.0 (.z (`self.VectorIteration_Spectate`))))))
          (else
            (set `self.SpecIter` 0)))))))

(event `InputAction|ZoomOut`
  (params (Key :type "Key Structure"))
  (bind _camera (`self.Camera`))
  ;[1 1 1] Movement
  ;;[0.03587 1 0] Zooming
  ;;;[0.03587 1 0 1 10] NOTE: because the camera isn't in perspective mode (otherwise moving player to mouse crusor looks off), changing z axis will not have any result. Changing orthograpic width however will if in orthographic mode. Look in camera's setting in Camera Component to change mode.
  (:`Pressed`
    (`CameraComponent.SetOrthoWidth` _camera (+ (`CameraComponent.OrthoWidth` _camera) (`self.ZoomValue`)))))

(event `Randomize Start`
  ;[0.7397 0 1] Randomize Function
  ;;[1 0 0.08382] Randomize Trigger
  (`|ExecutionSequence`
    (:`then_0`
      ;;[1 0.402 0] Button Count
      (set `self.ButtonCount` (+ (`self.ButtonCount`) (`self.PlayerButtonMultiplier`))))
    (:`then_1`
      (`KismetArrayLibrary.Array_Shuffle` (`self.SlotArray`)) ; Randomizes array
      (set `self.CrewPosition` (0.0 0.0 0.0)) ; Resets Crew Position
      (set `self.CurrentIndex_Crew` 0) ; Reset Current Index
      (`self.Randomizer`))))

(event `InputAction|ZoomIn`
  (params (Key :type "Key Structure"))
  (bind _camera (`self.Camera`))
  ;[1 1 1] Movement
  ;;[0.03587 1 0] Zooming
  ;;;[0.03587 1 0 1 10] NOTE: because the camera isn't in perspective mode (otherwise moving player to mouse crusor looks off), changing z axis will not have any result. Changing orthograpic width however will if in orthographic mode. Look in camera's setting in Camera Component to change mode.
  (:`Pressed`
    (`CameraComponent.SetOrthoWidth` _camera (- (`CameraComponent.OrthoWidth` _camera) (`self.ZoomValue`)))))

(event `InputAxis|MoveRight` :overrideparent false
  (params (AxisValue :type "Float (single-precision)"))
  ;[1 1 1] Movement
  ;;[0 1 0.003035] Panning With Keyboard
  (`self.AddMovementInput` (`KismetMathLibrary.GetRightVector` (`KismetMathLibrary.MakeRotator` 0.0 0.0 (.yaw (`self.GetControlRotation`)))) AxisValue))

(event `InputAction|Randomize`
  (params (Key :type "Key Structure"))
  ;[1 0.7712 0] Set Modes
  ;;[1 1 1] Randomize Toggles
  (:`Pressed`
    (set `self.PlayerButtonMultiplier` 1)
    (`self.Randomize Start`)
    (`self.Randomize End`)
    (`self.Spectator Randomizer`)
    (`self.SpecRandomizeEnd`)))

(event `/Game/Asset/BP/Core/BPI_UI.ApplyRandomize`
  ;[1 0.7712 0] Set Modes
  ;;[1 1 1] Runs Randomizer if called from Widget
  (`self.Randomize Start`)
  (`self.Randomize End`)
  (`self.Spectator Randomizer`)
  (`self.SpecRandomizeEnd`))

(event `Randomize End`
  ;[0.7397 0 1] Randomize Function
  ;;[1 0 0.08382] Randomize Trigger
  (goto _label_2 :!via `Reset`))

(event `InputAction|RandomizeX10`
  (params (Key :type "Key Structure"))
  ;[1 0.7712 0] Set Modes
  ;;[1 1 1] Randomize Toggles
  (:`Pressed`
    (set `self.PlayerButtonMultiplier` 10)
    (`self.Randomize Start`)
    (`self.Randomize End`)
    (`self.Spectator Randomizer`)
    (`self.SpecRandomizeEnd`)))

(event `SpecRandomizeEnd`
  ;[0.2785 0 1] Randomize Spectators
  ;;[1 1 1] Sorts Spectators into columns
  (goto _label :!via `Reset`))

(event `Key|Q`
  (params (Key :type "Key Structure"))
  ;[1 0.7712 0] Set Modes
  ;;[1 1 1] Toggle fps Stat
  (:`Pressed`
    (`KismetSystemLibrary.ExecuteConsoleCommand` "stat fps")))

(event `InputAction|Randomizex100`
  (params (Key :type "Key Structure"))
  ;[1 0.7712 0] Set Modes
  ;;[1 1 1] Randomize Toggles
  (:`Pressed`
    (set `self.PlayerButtonMultiplier` 100)
    (`self.Randomize Start`)
    (`self.Randomize End`)
    (`self.Spectator Randomizer`)
    (`self.SpecRandomizeEnd`)))

(event `InputAction|Mouse1Click`
  (params (Key :type "Key Structure"))
  ;[1 1 1] Movement
  ;;[0 1 0.003035] DISABLED: Panning With Mouse (left for future ref)
)

(event `/Game/Asset/BP/Core/BPI_UI.UIZoom`
  ;[1 1 1] Movement
  ;;[0 1 0.003035] Zooming With UI
  (`CameraComponent.SetOrthoWidth` (`self.Camera`) (* (`self.OrthoWidth`) (`self.UIZoomMultiplier`))))

(event `InputAction|Randomizex1000`
  (params (Key :type "Key Structure"))
  ;[1 0.7712 0] Set Modes
  ;;[1 1 1] Randomize Toggles
  (:`Pressed`
    (set `self.PlayerButtonMultiplier` 1000)
    (`self.Randomize Start`)
    (`self.Randomize End`)
    (`self.Spectator Randomizer`)
    (`self.SpecRandomizeEnd`)))

(event `Randomizer`
  (bind _output (`|GetArrayItem` (`self.SlotArray`) (`self.CurrentIndex_Crew`)))
  ;[0.7397 0 1] Randomize Function
  ;;[0 0.6625 1] Placing Crew Position
  (for _index (range (+ (`KismetArrayLibrary.Array_LastIndex` (`self.SlotArray`)) 1))
    (set `self.CurrentIndex_Crew` _index)
    (`|ExecutionSequence`
      (:`then_0`
        ;;;[1 1 1] Set Crew Position
        (`self.K2_SetActorLocation` _output (+ (`self.CrewPosition`) (`self.VectorIteration_Crew`)) false false)
        (set `self.CrewPosition` (`self.K2_GetActorLocation` _output)))
      (:`then_1`
        ;;;[1 1 1] Group Ships to Fleet
        (if (>= (`self.CurrentIndex_Crew`) 15)
          (`/Engine/EditorBlueprintResources/StandardMacros.DoOnce` false :!label _label_2
            (:`Completed`
              (set `self.CrewPosition` (300.0 0.0 0.0)) ; Reset Crew Position with an column offset
            ))
          (else
            (`/Engine/EditorBlueprintResources/StandardMacros.DoOnce` false))))
      (:`then_2`
        ;;;[1 1 1] Group Crew to Ship
        (if (!= (`self.CrewIter`) 3)
          (bind _counter (`/Engine/EditorBlueprintResources/StandardMacros.Do N` 3 :!label _label_3)
            (:`Exit`
              (set `self.CrewIter` _counter)
              (set `self.VectorIteration_Crew` (`KismetMathLibrary.MakeVector` (.x (`self.VectorIteration_Crew`)) 25.0 (.z (`self.VectorIteration_Crew`))))))
          (else
            (set `self.CrewIter` 0)
            (set `self.VectorIteration_Crew` (`KismetMathLibrary.MakeVector` (.x (`self.VectorIteration_Crew`)) 75.0 (.z (`self.VectorIteration_Crew`))))
            (goto _label_3 :!via `Reset`)))))))

(event `/Game/Asset/BP/Core/BPI_UI.UIxPan`
  (bind (_returnvalue_x _returnvalue_y _returnvalue_z) (`KismetMathLibrary.BreakVector` (`self.K2_GetActorLocation`)))
  ;[1 1 1] Movement
  ;;[0 1 0.003035] Panning With UI
  ;;;[0 1 0.003035] X Panning
  (`self.K2_SetActorLocation` (`KismetMathLibrary.MakeVector` (+ (* (`self.XPanning`) (`self.UIPannerMultiplier`)) _returnvalue_x) _returnvalue_y _returnvalue_z) false true))

(event `/Game/Asset/BP/Core/BPI_UI.UIyPan`
  (bind (_returnvalue_x _returnvalue_y _returnvalue_z) (`KismetMathLibrary.BreakVector` (`self.K2_GetActorLocation`)))
  ;[1 1 1] Movement
  ;;[0 1 0.003035] Panning With UI
  ;;;[0 1 0.003035] Y Panning
  (`self.K2_SetActorLocation` (`KismetMathLibrary.MakeVector` _returnvalue_x (+ (* (`self.YPanning`) (`self.UIPannerMultiplier`)) _returnvalue_y) _returnvalue_z) false true))

(event `/Game/Asset/BP/Core/BPI_UI.PetriPilotToggle`
  ;[1 0.9635 0.002934] Petri Pilot Toggle
  (`/Engine/EditorBlueprintResources/StandardMacros.FlipFlop`
    (:`A`
      (set `self.PetriVisiblityCoords` 500.0))
    (:`B`
      (set `self.PetriVisiblityCoords` -1000.0)))
  (`self.PetriPilotVisibility`))

(event `PetriPilotVisibility`
  (bind _output (`|GetArrayItem` (`self.PetriArray`) (`self.CurrentIndex_Petri`)))
  (bind (_returnvalue_x _returnvalue_y) (`KismetMathLibrary.BreakVector` (`self.K2_GetActorLocation` _output)))
  ;[1 0.9635 0.002934] Petri Pilot Toggle
  ;;[0 0.6625 1] Placing Petri
  (for _index (range (+ (`KismetArrayLibrary.Array_LastIndex` (`self.PetriArray`)) 1))
    (set `self.CurrentIndex_Petri` _index)
    (`self.K2_SetActorLocation` _output (+ (`self.PetriPosition`) (`KismetMathLibrary.MakeVector` _returnvalue_x _returnvalue_y (`self.PetriVisiblityCoords`))) false false)))

(fn `UserConstructionScript`
  (`|ExecutionSequence`
    (:`then_0`
      (bind _outactors (`GameplayStatics.GetAllActorsOfClass` "/Game/Asset/BP/Core/BP_Crew.BP_Crew_C"))
      (bind _output_get (set `self.SlotArray` _outactors))
      (`KismetArrayLibrary.Array_Shuffle` _output_get))
    (:`then_1`
      (bind _outactors_2 (`GameplayStatics.GetAllActorsOfClass` "/Game/Asset/BP/Core/BP_Spectate.BP_Spectate_C"))
      (bind _output_get_2 (set `self.SpecArray` _outactors_2))
      (`KismetArrayLibrary.Array_Shuffle` _output_get_2))
    (:`then_2`
      (bind _outactors_3 (`GameplayStatics.GetAllActorsOfClass` "/Game/Asset/BP/Core/BP_Petri.BP_Petri_C"))
      (set `self.PetriArray` _outactors_3))))